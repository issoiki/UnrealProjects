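; Player controller that owns the game's main UI, pause menu and death screen, and starts the clown music.
; BeginPlay adds the main widget and binds to the character health component's death event.
; On death, a one-shot handler shows the death screen with UI-only input and saves the score through the game instance.
; Escape toggles pause, widget and input mode inline, largely duplicating ToggleEscapeMenu, which differs in hiding the cursor on resume.
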(event Custom|OnCharDead
  (if (not (Variables|Default|GetCharDead))
    (Variables|Default|SetCharDead true)
    (Variables|Default|SetbShowMouseCursor true)
    (Input|SetInputModeUIOnly self 0 "DoNotLock")
    (bind _returnvalue (UserInterface|CreateWidget "/Game/UI/OnDeath/WD_OnDeath.WD_OnDeath_C"))
    (bind _output_get (Variables|Default|SetWD_OnDeath _returnvalue))
    (UserInterface|Viewport|AddtoViewport _output_get 0)
    (Default|SaveScore (.AsBP%20Game%20Instance (Utilities|Casting|CastToBP_GameInstance (Game|GetGameInstance))))))

(event EventBeginPlay
  (Variables|Default|SetPlayerCharacter (.AsBP%20Player%20Character (Utilities|Casting|CastToBP_PlayerCharacter (Game|Player|GetPlayerPawn 0))))
  (bind _returnvalue (UserInterface|CreateWidget "/Game/UI/InGame/WD_Main.WD_Main_C"))
  (bind _output_get (Variables|Default|SetWD_Main _returnvalue))
  (UserInterface|Viewport|AddtoViewport _output_get 0)
  (EventDispatchers|BindEventtoCharDead (Variables|/Game/Blueprints/Character/BP_PlayerCharacter.BP_PlayerCharacter_C|GetBP_HealthComponent (Variables|Default|GetPlayerCharacter)) (EventDispatchers|CreateEvent :!event Custom|OnCharDead))
  (Audio|PlaySound2D "/Game/Assets/Sounds/Music/ClownMusic_Cue.ClownMusic_Cue" 1.0 1.0 0.0 0 0))

(event Input|KeyboardEvents|Escape
  (params (Key :type Key%20Structure :default "None"))
  (:Pressed
    (if (Variables|Default|GetGameisPaused)
      (bind _wd_pause (Variables|Default|GetWD_Pause)
        (:then
          (Widget|RemovefromParent _wd_pause)
          (Game|SetGamePaused false)
          (Variables|Default|SetGameisPaused false)
          (Variables|Default|SetbShowMouseCursor true)
          (Input|SetInputModeGameOnly self))
        (:else))
      (else
        (bind _returnvalue (UserInterface|CreateWidget "/Game/UI/InGame/WD_Pause.WD_Pause_C"))
        (bind _output_get (Variables|Default|SetWD_Pause _returnvalue))
        (UserInterface|Viewport|AddtoViewport _output_get 0)
        (Game|SetGamePaused true)
        (Variables|Default|SetGameisPaused true)
        (Variables|Default|SetbShowMouseCursor true)
        (Input|SetInputModeUIOnly self 0 "DoNotLock")))))

(fn ConstructionScript)

(fn ToggleEscapeMenu
  (params (TurnOn? :type Boolean))
  (if TurnOn?
    (bind _returnvalue (UserInterface|CreateWidget "/Game/UI/InGame/WD_Pause.WD_Pause_C"))
    (bind _output_get (Variables|Default|SetWD_Pause _returnvalue))
    (UserInterface|Viewport|AddtoViewport _output_get 0)
    (Game|SetGamePaused true)
    (Variables|Default|SetGameisPaused true)
    (Variables|Default|SetbShowMouseCursor true)
    (Input|SetInputModeUIOnly self 0 "DoNotLock")
    (else
      (bind _wd_pause (Variables|Default|GetWD_Pause)
        (:then
          (Widget|RemovefromParent _wd_pause)
          (Game|SetGamePaused false)
          (Variables|Default|SetGameisPaused false)
          (Variables|Default|SetbShowMouseCursor false)
          (Input|SetInputModeGameOnly self))
        (:else)))))