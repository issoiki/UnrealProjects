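; BP_HealthComponent is a player component that tracks health and signals death.
; On BeginPlay it resets health, casts player 0's pawn to BP_PlayerCharacter rather than using its owner, and binds to that character's point damage event.
; Each hit subtracts damage from CurrentHealth and calls CharDead whenever the result is zero or below.
; The IsDead? function is an empty stub.
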(event Custom|PlayerTakeDamage
  (params (DamagedActor :type Actor%20Object%20Reference) (Damage :type Float%20%28single-precision%29) (InstigatedBy :type Controller%20Object%20Reference) (HitLocation :type Vector) (FHitComponent :type Primitive%20Component%20Object%20Reference) (BoneName :type Name) (ShotFromDirection :type Vector) (DamageType :type Damage%20Type%20Object%20Reference) (DamageCauser :type Actor%20Object%20Reference))
  (bind _output_get (Variables|Default|SetCurrentHealth (- (Variables|Default|GetCurrentHealth) Damage)))
  (if (<= _output_get 0.0)
    (Default|CallCharDead)))

(event EventBeginPlay
  (Variables|Default|SetCurrentHealth 1.0)
  (bind _output_get (Variables|Default|SetPlayerCharacter (.AsBP%20Player%20Character (Utilities|Casting|CastToBP_PlayerCharacter (Game|GetPlayerCharacter 0)))))
  (EventDispatchers|BindEventtoOnTakePointDamage _output_get (EventDispatchers|CreateEvent :!event Custom|PlayerTakeDamage)))

(fn IsDead?)