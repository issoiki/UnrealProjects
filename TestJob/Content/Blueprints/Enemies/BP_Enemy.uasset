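; Enemy character that chases the player through AI perception and deals contact damage.
; The ProcessStimuli macro filters perception stimuli to Player-tagged actors and writes sensed ones to the blackboard follow target; losing track calls an empty stub.
; Capsule overlaps track whether the player is in range and store the last hit.
; Tick applies point damage while in range, gated by a Delay-based cooldown.
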(event OnTargetPerceptionUpdated(AIPerception)
  (params (Actor :type Actor%20Object%20Reference) (Stimulus :type AI%20Stimulus%20Structure))
  ;[1 1 1] PawnSensing
  (Utilities|ProcessStimuli Actor Stimulus
    (:FollowNewActor
      (CallFunction|FollowNewActorTarget Actor))
    (:LostTrackOfTarget
      (CallFunction|LostTrackOfTarget))))

(event OnComponentBeginOverlap(CapsuleComponent)
  (params (OverlappedComponent :type Primitive%20Component%20Object%20Reference) (OtherActor :type Actor%20Object%20Reference) (OtherComp :type Primitive%20Component%20Object%20Reference) (OtherBodyIndex :type Integer) (bFromSweep :type Boolean) (SweepResult :type Hit%20Result%20Structure%20%28by%20ref%29))
  ;[1 1 1] ApplyingDamageToPlayer
  (Utilities|Casting|CastToBP_PlayerCharacter OtherActor)
  (Variables|Default|SetLastHitResult SweepResult)
  (Variables|Default|SetInRadiusForPlayer true))

(event OnComponentEndOverlap(CapsuleComponent)
  (params (OverlappedComponent :type Primitive%20Component%20Object%20Reference) (OtherActor :type Actor%20Object%20Reference) (OtherComp :type Primitive%20Component%20Object%20Reference) (OtherBodyIndex :type Integer))
  ;[1 1 1] ApplyingDamageToPlayer
  (Utilities|Casting|CastToBP_PlayerCharacter OtherActor)
  (Variables|Default|SetInRadiusForPlayer false))

(event EventTick
  (params (DeltaSeconds :type Float%20%28single-precision%29))
  (if (Variables|Default|GetInRadiusForPlayer)
    (if (Variables|Default|GetCanDamagePlayer?)
      (CallFunction|DamagePlayer)
      (Variables|Default|SetCanDamagePlayer? false)
      (Utilities|FlowControl|Delay 2.0)
      (Variables|Default|SetCanDamagePlayer? true))))

(fn ConstructionScript)

(fn FollowNewActorTarget
  (params (TargetToFollow :type Object%20Object%20Reference))
  (AI|Components|Blackboard|SetValueasObject (AI|GetBlackboard self) (Variables|Default|GetFollowTargetKey) TargetToFollow)
  (return))

(fn LostTrackOfTarget)

(fn DamagePlayer
  (bind _self self)
  (if (Variables|Default|GetCanDamagePlayer?)
    (Game|Damage|ApplyPointDamage (.AsBP%20Player%20Character (Utilities|Casting|CastToBP_PlayerCharacter (Game|GetPlayerCharacter 0))) 0.25 (Transformation|GetActorLocation) (Variables|Default|GetLastHitResult) (Pawn|GetController _self) _self)))