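; BP_AI_HealthComponent is an actor component that handles health, hit scoring and death for BP_Enemy.
; On BeginPlay it binds to the owner's point damage event and caches the game instance and game mode.
; Each hit spawns an explosion and ignores incoming damage, applying fixed health loss and score, both higher for head-sphere hits.
; At zero health it calls SpawnEnemies on BP_Gamemode and destroys the enemy.
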(event Custom|OnEnemyTakePointDamage
  (params (DamagedActor :type Actor%20Object%20Reference) (Damage :type Float%20%28single-precision%29) (InstigatedBy :type Controller%20Object%20Reference) (HitLocation :type Vector) (FHitComponent :type Primitive%20Component%20Object%20Reference) (BoneName :type Name) (ShotFromDirection :type Vector) (DamageType :type Damage%20Type%20Object%20Reference) (DamageCauser :type Actor%20Object%20Reference))
  (bind _gameinstance (Variables|Default|GetGameInstance))
  (Effects|SpawnEmitteratLocation "/Game/Assets/StarterContent/Particles/P_Explosion.P_Explosion" HitLocation (Math|Rotator|FindLookatRotation HitLocation ShotFromDirection))
  (if (== FHitComponent (Variables|/Game/Blueprints/Enemies/BP_Enemy.BP_Enemy_C|GetSphere (Variables|Default|GetPawn)))
    (Variables|Default|SetCurrentHealth (- (Variables|Default|GetCurrentHealth) 0.5))
    (Default|EditScore _gameinstance 40)
    (else
      (Variables|Default|SetCurrentHealth (- (Variables|Default|GetCurrentHealth) 0.2))
      (Default|EditScore _gameinstance 10)))
  (if (<= (Variables|Default|GetCurrentHealth) 0.0)
    (Default|SpawnEnemies (Variables|Default|GetGamemode) false)
    (Actor|DestroyActor (Variables|Default|GetPawn))))

(event EventBeginPlay
  (Variables|Default|SetCurrentHealth 1.0)
  (bind _asbp_enemy (Utilities|Casting|CastToBP_Enemy (Components|GetOwner)))
  (bind _output_get (Variables|Default|SetPawn _asbp_enemy))
  (EventDispatchers|BindEventtoOnTakePointDamage _output_get (EventDispatchers|CreateEvent :!event Custom|OnEnemyTakePointDamage))
  (Variables|Default|SetGameInstance (.AsBP%20Game%20Instance (Utilities|Casting|CastToBP_GameInstance (Game|GetGameInstance))))
  (Variables|Default|SetGamemode (.AsBP%20Gamemode (Utilities|Casting|CastToBP_Gamemode (Game|GetGameMode)))))

(event EventTick
  (params (DeltaSeconds :type Float%20%28single-precision%29)))

(fn UpdateScoreinInstance
  (params (ScoreToAdd :type Integer))
  (bind _asbp_game_instance (Utilities|Casting|CastToBP_GameInstance (Game|GetGameInstance)))
  (Variables|/Game/Blueprints/Game/BP_GameInstance.BP_GameInstance_C|SetScore _asbp_game_instance (+ (Variables|/Game/Blueprints/Game/BP_GameInstance.BP_GameInstance_C|GetScore _asbp_game_instance) ScoreToAdd)))