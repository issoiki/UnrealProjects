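; BP_Gamemode is a game mode Blueprint that resets the score and controls enemy spawning at spawn points.
; On BeginPlay it zeroes the Score in BP_GameInstance, caches all BP_SpawnPoint actors, then spawns at every point after a short delay.
; SpawnEnemies also has a non-start mode that twice shuffles the points and spawns at the first, so the same point can repeat.
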(event EventBeginPlay
  (Utilities|FlowControl|Sequence
    (:then_0
      (CallFunction|SetInstanceScoretoZero)
      (bind _outactors (Actor|GetAllActorsOfClass "/Game/Blueprints/Game/SpawnEnemiesThings/BP_SpawnPoint.BP_SpawnPoint_C"))
      (Variables|Default|SetSpawnPoints _outactors))
    (:then_1
      (Utilities|FlowControl|Delay 2.0)
      (CallFunction|SpawnEnemies true))))

(fn ConstructionScript)

(fn SpawnEnemies
  (params (StartMap? :type Boolean))
  (bind _spawnpoints (Variables|Default|GetSpawnPoints))
  (bind _output (Utilities|Array|Get(acopy) _spawnpoints))
  (if StartMap?
    (bind _array_element (Utilities|Array|ForEachLoopwithBreak (Variables|Default|GetSpawnPoints))
      (:LoopBody
        (Default|SpawnEnemy _array_element)))
    (else
      (for _index (range 0 1)
        (Utilities|Array|Shuffle (Variables|Default|GetSpawnPoints))
        (Utilities|IsValid _output
          (:Is%20Valid
            (Default|SpawnEnemy _output)))))))

(fn SetInstanceScoretoZero
  (bind _asbp_game_instance (Utilities|Casting|CastToBP_GameInstance (Game|GetGameInstance)))
  (Variables|/Game/Blueprints/Game/BP_GameInstance.BP_GameInstance_C|SetScore _asbp_game_instance 0))