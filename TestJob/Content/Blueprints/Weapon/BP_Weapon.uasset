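; BP_Weapon is a hitscan gun for the first-person player character.
; On BeginPlay it caches player 0's BP_PlayerCharacter to use its camera for aiming.
; Shooting line traces from the muzzle socket along the camera's forward vector, applies point damage to the hit actor and plays a gunshot sound at the muzzle.
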(event EventBeginPlay
  (Variables|Default|SetPlayerCharacter (.AsBP%20Player%20Character (Utilities|Casting|CastToBP_PlayerCharacter (Game|GetPlayerCharacter 0)))))

(fn ConstructionScript)

(fn Shooting
  (bind _skeletalmesh (Variables|Default|GetSkeletalMesh))
  (bind _skeletalmesh_2 (Variables|Default|GetSkeletalMesh))
  (bind _returnvalue (Transformation|GetSocketTransform _skeletalmesh "SKT_Muzzle" "RTS_World"))
  (bind _returnvalue_2 (Transformation|GetSocketTransform _skeletalmesh_2 "SKT_Muzzle" "RTS_World"))
  (bind _location (Math|Transform|BreakTransform _returnvalue))
  (bind (_location_2 _rotation) (Math|Transform|BreakTransform _returnvalue_2))
  (bind _outhit (Collision|LineTraceByChannel _location (+ (* (Math|Vector|GetForwardVector (Variables|/Game/Blueprints/Character/BP_PlayerCharacter.BP_PlayerCharacter_C|GetFirstPersonCamera (Variables|Default|GetPlayerCharacter))) 5e+03) _location) "TraceTypeQuery1" false 0 "None"))
  (Game|Damage|ApplyPointDamage (.HitActor (Collision|BreakHitResult _outhit)) 5.0 (Math|Vector|GetUnitDirection(Vector) (.TraceEnd (Collision|BreakHitResult _outhit)) (.TraceStart (Collision|BreakHitResult _outhit))) _outhit (Game|GetInstigatorController) self)
  (Audio|PlaySoundatLocation "/Game/Assets/Sounds/SFX/gun-gunshot-02_Cue.gun-gunshot-02_Cue" _location_2 _rotation 1.0 1.0 0.0 0 0 0))